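; KeyBox is a Blueprint actor that raises and lowers its static mesh through GoUp and GoDown events.
; BeginPlay caches the actor's location and rotation as the starting target.
; Each event shifts that stored target along Z by a fixed step, sets IsUp and eases the mesh over time with MoveComponentTo.
; The cached world-space values are passed as relative targets, and neither event checks IsUp before moving.
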(event Custom|GoDown
  ;[1 1 1] Move Down
  (bind _output_get (Variables|Default|SetTargetLocation (+ (Variables|Default|GetTargetLocation) "0, 0,-70.000000")))
  (Variables|Default|SetIsUp false)
  (Components|MoveComponentTo (Variables|Debug|GetStaticMeshComponent) _output_get (Variables|Default|GetRotation) false false 2.0 false))

(event Custom|GoUp
  ;[1 1 1] Move Up
  (bind _output_get (Variables|Default|SetTargetLocation (+ (Variables|Default|GetTargetLocation) "0, 0,70.000000")))
  (Variables|Default|SetIsUp true)
  (Components|MoveComponentTo (Variables|Debug|GetStaticMeshComponent) _output_get (Variables|Default|GetRotation) false false 2.0 false))

(event EventBeginPlay
  (Variables|Default|SetTargetLocation (Transformation|GetActorLocation))
  (Variables|Default|SetRotation (Transformation|GetActorRotation)))

(fn ConstructionScript)