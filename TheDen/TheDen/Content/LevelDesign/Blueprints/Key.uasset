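; Key is a pickup actor that adds an item to the player's inventory when the player character walks into its box.
; On overlap it casts to the character and its LD_playerController, then adds PickupItem to that Inventory without duplicates.
; If RemoveAfterPickup is set, it flags its PickupNumber in the PickedUp array of the game mode cached at BeginPlay, then destroys itself.
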(event OnComponentBeginOverlap(Box)
  (params (OverlappedComponent :type Primitive%20Component%20Object%20Reference) (OtherActor :type Actor%20Object%20Reference) (OtherComp :type Primitive%20Component%20Object%20Reference) (OtherBodyIndex :type Integer) (bFromSweep :type Boolean) (SweepResult :type Hit%20Result%20Structure%20%28by%20ref%29))
  (bind _asthird_person_character (Utilities|Casting|CastToThirdPersonCharacter OtherActor)) ; Was it a player character?
  ;[1 1 1] Get the controller for the player character
  (bind _asld_player_controller (Utilities|Casting|CastToLD_playerController (Pawn|GetController _asthird_person_character)))
  ;[1 1 1] Add item to the player inventory
  (Utilities|Array|AddUnique (Variables|/Game/LevelDesign/LD_playerController.LD_playerController_C|GetInventory _asld_player_controller) (Variables|Default|GetPickupItem))
  ;[1 1 1] Does the pickup disapear?
  (if (Variables|Default|GetRemoveAfterPickup)
    (Utilities|Array|SetArrayElem (Variables|/Game/ThirdPersonBP/Blueprints/ThirdPersonGameMode.ThirdPersonGameMode_C|GetPickedUp (Variables|Default|GetGameMode)) (Variables|Default|GetPickupNumber) true)
    (Actor|DestroyActor)))

(event EventBeginPlay
  (bind _asthird_person_game_mode (Utilities|Casting|CastToThirdPersonGameMode (Game|GetGameMode)))
  (Variables|Default|SetGameMode _asthird_person_game_mode))

(fn ConstructionScript)