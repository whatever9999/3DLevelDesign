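; Door Blueprint that slides up when a player character enters its trigger and lowers again when that character leaves.
; On overlap it either opens directly or, depending on DoorRequires, first checks the LD_playerController inventory for the required item.
; MoveComponentTo moves the Door component between fixed relative positions over a short time.
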(event OnComponentEndOverlap(Trigger)
  (params (OverlappedComponent :type Primitive%20Component%20Object%20Reference) (OtherActor :type Actor%20Object%20Reference) (OtherComp :type Primitive%20Component%20Object%20Reference) (OtherBodyIndex :type Integer))
  (Utilities|Casting|CastToThirdPersonCharacter OtherActor) ; Was it a player character?
  (Components|MoveComponentTo (Variables|Default|GetDoor) "0, 0,0.000000" "0, 0, 0" false false 0.2 false))

(event OnComponentBeginOverlap(Trigger)
  (params (OverlappedComponent :type Primitive%20Component%20Object%20Reference) (OtherActor :type Actor%20Object%20Reference) (OtherComp :type Primitive%20Component%20Object%20Reference) (OtherBodyIndex :type Integer) (bFromSweep :type Boolean) (SweepResult :type Hit%20Result%20Structure%20%28by%20ref%29))
  (bind _asthird_person_character (Utilities|Casting|CastToThirdPersonCharacter OtherActor)) ; Was it a player character?
  ;[1 1 1] Get the controller for the player character
  (bind _asld_player_controller (Utilities|Casting|CastToLD_playerController (Pawn|GetController _asthird_person_character)))
  ;[1 1 1] Does the door open on void
  (if (Utilities|Enum|Equal(Enum) (Variables|Default|GetDoorRequires) "NewEnumerator1") ; Does door require an item
    (Utilities|FlowControl|Sequence :!label _label
      (:then_0
        (Components|MoveComponentTo (Variables|Default|GetDoor) "0.000000, 0,188.000000" "0, 0, 0" false false 0.2 false)))
    (else
      ;[1 1 1] Check the inventory for an item
      (if (Utilities|Array|ContainsItem (Variables|/Game/LevelDesign/LD_playerController.LD_playerController_C|GetInventory _asld_player_controller) (Variables|Default|GetDoorRequires))
        (goto _label)))))

(fn ConstructionScript)